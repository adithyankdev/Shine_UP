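; Obstacle actor that shuttles endlessly back and forth between two location points, starting on BeginPlay.
; A Timeline drives a lerp of its relative location from LocationPoint2 to LocationPoint1, without sweeping for collisions.
; Each time the Timeline finishes, the actor turns 180 degrees in yaw.
; The Reverse flag then toggles and, after a one-tick delay, restarts the Timeline forward or backward.
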(event EventBeginPlay
  (bind _returnvalue (Transformation|GetActorRotation))
  (bind _newtrack_0 (Timeline|Timeline PlayFromStart)
    (:Update
      (Transformation|SetActorRelativeLocation (Math|Vector|Lerp(Vector) (Variables|Default|GetLocationPoint2) (Variables|Default|GetLocationPoint1) _newtrack_0)))
    (:Finished
      (Transformation|SetActorRotation (Math|Rotator|MakeRotator (.roll _returnvalue) (.pitch _returnvalue) (+ (.yaw _returnvalue) 1.8e+02)))
      (if (Variables|Default|Getreverse)
        (Utilities|FlowControl|DelayUntilNextTick)
        (Variables|Default|Setreverse false)
        (Timeline|Timeline PlayFromStart)
        (else
          (Utilities|FlowControl|DelayUntilNextTick)
          (Variables|Default|Setreverse true)
          (Timeline|Timeline ReverseFromEnd))))))

(event Collision|EventActorBeginOverlap
  (params (OtherActor :type Actor%20Object%20Reference)))

(event EventTick
  (params (DeltaSeconds :type Float%20%28single-precision%29)))

(fn ConstructionScript)